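; Movement component that gives the owning character stamina-limited sprinting and crouching by changing its max walk speed.
; Looping timers drain stamina while sprinting and moving, then regenerate it after a retriggerable five-second delay once sprinting stops.
; Crouching cancels the sprint timer and has CABINCharacter resize its capsule, while starting a sprint ends any crouch.
; Initialize supplies the character reference, and stamina changes are printed on screen.
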(event `StartSprint`
  (if (`self.IsCrouching`)
    (`self.EndCrouch`))
  (if (and (> (`self.CurrStamina`) (`self.MinStamina`)) (> (`KismetMathLibrary.VSize` (`Actor.GetVelocity` (`self.Character`))) 10.0))
    (`KismetSystemLibrary.K2_ClearTimer` null "RegenerateStamina")
    (`self.Set Player Max Walk Speed` (`self.SprintSpeed`))
    (`KismetSystemLibrary.K2_SetTimer` null "SprintTimer" (`self.LossSpeed`) true)))

(event `SprintTimer`
  (if (> (`KismetMathLibrary.VSize` (`Actor.GetVelocity` (`self.Character`))) 10.0)
    (bind _output_get (set `self.CurrStamina` (`KismetMathLibrary.FClamp` (- (`self.CurrStamina`) 1.0) (`self.MinStamina`) (`self.MaxStamina`))))
    (`KismetSystemLibrary.PrintString` (`KismetStringLibrary.Conv_DoubleToString` _output_get))
    (if (<= (`self.CurrStamina`) (`self.MinStamina`))
      (`self.SprintStop`))
    (else
      (`self.SprintStop`))))

(event `SprintStop`
  (if (not (`self.IsCrouching`))
    (`KismetSystemLibrary.K2_ClearTimer` null "SprintTimer")
    (`self.Set Player Max Walk Speed` (`self.WalkSpeed`))
    (`KismetSystemLibrary.RetriggerableDelay` 5.0)
    (if (not (`KismetSystemLibrary.K2_IsTimerActive` null "SprintTimer"))
      (`KismetSystemLibrary.K2_SetTimer` null "RegenerateStamina" (`self.RegenSpeed`) true))))

(event `RegenerateStamina`
  (bind _output_get (set `self.CurrStamina` (`KismetMathLibrary.FClamp` (+ (`self.CurrStamina`) 1.0) (`self.MinStamina`) (`self.MaxStamina`))))
  (`KismetSystemLibrary.PrintString` (`KismetStringLibrary.Conv_DoubleToString` _output_get))
  (if (>= (`self.CurrStamina`) (`self.MaxStamina`))
    (`KismetSystemLibrary.K2_ClearTimer` null "RegenerateStamina")))

(event `StartCrouch`
  (`KismetSystemLibrary.K2_ClearTimer` null "SprintTimer")
  (`self.Set Player Max Walk Speed` (`self.CrouchSpeed`))
  (`/Game/GameBP/Tutorial/CABINCharacter.ShortenPlayerCapsule` (cast `/Game/GameBP/Tutorial/CABINCharacter` (`self.Character`) :!pure true))
  (set `self.IsCrouching` true))

(event `EndCrouch`
  (`self.Set Player Max Walk Speed` (`self.WalkSpeed`))
  (`/Game/GameBP/Tutorial/CABINCharacter.LengthenPlayerCapsule` (cast `/Game/GameBP/Tutorial/CABINCharacter` (`self.Character`) :!pure true))
  (set `self.IsCrouching` false))

(fn `Initialize`
  (params (Character :type "Character Object Reference"))
  (set `self.Character` Character)
  (set `CharacterMovementComponent.MaxWalkSpeed` (`self.WalkSpeed`) (`Character.CharacterMovement` (`self.Character`))))

(fn `Set Player Max Walk Speed`
  (params (MaxWalkSpeed :type "Float (single-precision)"))
  (set `CharacterMovementComponent.MaxWalkSpeed` MaxWalkSpeed (`Character.CharacterMovement` (`self.Character`))))